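; BP_BallDoor is a door actor that swings to a fixed rotation when any overlap with its Box ends.
; BeginPlay stores the root's starting rotation and speeds up a Timeline, which lerps the root between that rotation and a hardcoded end rotation.
; The Open event reverses the Timeline, so the starting pose acts as the open state and leaving the box shuts the door.
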(event OnComponentEndOverlap(Box)
  (params (OverlappedComponent :type Primitive%20Component%20Object%20Reference) (OtherActor :type Actor%20Object%20Reference) (OtherComp :type Primitive%20Component%20Object%20Reference) (OtherBodyIndex :type Integer))
  (bind _newtrack_0 (Timeline|Timeline Play)
    (:Update
      (Transformation|SetRelativeRotation (Variables|Default|GetDefaultSceneRoot) (Math|Rotator|Lerp(Rotator) (Variables|Default|GetStartRot) (Variables|Default|GetEndRot) _newtrack_0) false false))))

(event Custom|Open
  (bind _newtrack_0 (Timeline|Timeline Reverse)
    (:Update
      (Transformation|SetRelativeRotation (Variables|Default|GetDefaultSceneRoot) (Math|Rotator|Lerp(Rotator) (Variables|Default|GetStartRot) (Variables|Default|GetEndRot) _newtrack_0) false false))))

(event EventBeginPlay
  (Variables|Default|SetStartRot (Transformation|GetWorldRotation (Variables|Default|GetDefaultSceneRoot)))
  (Variables|Default|SetEndRot "41.000000,-90.000000,0.000000")
  (Components|Timeline|SetPlayRate (Variables|Default|GetTimeline) 5.0))

(event Collision|EventActorBeginOverlap
  (params (OtherActor :type Actor%20Object%20Reference)))

(event EventTick
  (params (DeltaSeconds :type Float%20%28single-precision%29)))

(fn ConstructionScript)