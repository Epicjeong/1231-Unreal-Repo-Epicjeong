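; Pinball game state Blueprint that tracks the score and the number of balls left.
; BeginPlay resets the score and sets the starting ball count.
; SetScore and HandleBalls events overwrite their value, then call the OnScoreChanged and OnBallsLost dispatchers to notify listeners.
; Each change, and the initial state, is also printed for debugging.
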(event Custom|SetScore
  (params (NewScore :type Float%20%28double-precision%29))
  (bind _output_get (Variables|Default|SetScore NewScore))
  (Default|CallOnScoreChanged _output_get)
  (Development|PrintString (Utilities|String|ToString(Float) _output_get)))

(event Custom|HandleBalls
  (params (HandleBalls :type Integer))
  (bind _output_get (Variables|Default|SetBallsLeft HandleBalls))
  (Default|CallOnBallsLost _output_get)
  (Development|PrintString (Utilities|String|ToString(Integer) _output_get)))

(event EventBeginPlay
  (bind _output_get (Variables|Default|SetScore 0.0))
  (bind _output_get_2 (Variables|Default|SetBallsLeft 9))
  (Development|PrintString (Utilities|String|ToString(Integer) _output_get_2))
  (Development|PrintString (Utilities|String|ToString(Float) _output_get)))

(event EventTick
  (params (DeltaSeconds :type Float%20%28single-precision%29)))

(fn ConstructionScript)