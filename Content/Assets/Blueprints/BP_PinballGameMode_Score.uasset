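; Score-based pinball game mode that adds points and handles lost balls through to game over.
; An AddScore event increases the score stored in BP_PinballGameState.
; OnBallLost extends the parent logic, passes the decremented ball count to the game state, then respawns through BP_PinballGameMode_Base while balls remain.
; With none left, it shows WBP_GameOver with the final score.
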(event EventBeginPlay
  (|CallParentFunction))

(event EventTick
  (params (DeltaSeconds :type Float%20%28single-precision%29))
  (|CallParentFunction DeltaSeconds) ; This node is disabled and will not be called.\nDrag off pins to build functionality.
)

(event EventAddScore
  (params (Points :type Float%20%28double-precision%29))
  (bind _asbp_pinball_game_state (Utilities|Casting|CastToBP_PinballGameState (Game|GetGameState)))
  (Default|SetScore _asbp_pinball_game_state (+ (Variables|/Game/Assets/Blueprints/BP_PinballGameState.BP_PinballGameState_C|GetScore _asbp_pinball_game_state) Points)))

(fn ConstructionScript
  (|CallParentFunction))

(fn OnBallLost
  (|CallParentFunction)
  (bind _asbp_pinball_game_state (Utilities|Casting|CastToBP_PinballGameState (Game|GetGameState)))
  (Default|HandleBalls _asbp_pinball_game_state (- (Variables|/Game/Assets/Blueprints/BP_PinballGameState.BP_PinballGameState_C|GetBallsLeft _asbp_pinball_game_state) 1))
  (if (> (Variables|/Game/Assets/Blueprints/BP_PinballGameState.BP_PinballGameState_C|GetBallsLeft _asbp_pinball_game_state) 0)
    (bind _asbp_pinball_game_mode_base (Utilities|Casting|CastToBP_PinballGameMode_Base (Game|GetGameMode)))
    (Default|SpawnBall _asbp_pinball_game_mode_base)
    (else
      (bind _returnvalue (UserInterface|CreateWidget "/Game/Assets/Widgets/WBP_GameOver.WBP_GameOver_C"))
      (UserInterface|Viewport|AddtoViewport _returnvalue 0)
      (Default|SetFinalText _returnvalue (Variables|/Game/Assets/Blueprints/BP_PinballGameState.BP_PinballGameState_C|GetScore _asbp_pinball_game_state)))))