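; BP_Bumper is a pinball bumper that knocks reactive objects away and awards points when they touch it.
; On sphere overlap it sends an impulse through BPI_PinballReactive, directed from the bumper toward the overlapping component and scaled by BumpStrength.
; It then prints a leftover debug string and passes PointValue to the game mode if that implements BPI_ScoreReciever.
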(event OnComponentBeginOverlap(Sphere)
  (params (OverlappedComponent :type Primitive%20Component%20Object%20Reference) (OtherActor :type Actor%20Object%20Reference) (OtherComp :type Primitive%20Component%20Object%20Reference) (OtherBodyIndex :type Integer) (bFromSweep :type Boolean) (SweepResult :type Hit%20Result%20Structure%20%28by%20ref%29))
  (bind _returnvalue (Game|GetGameMode))
  (bind _asbpi_pinball_reactive (Utilities|Casting|CastToBPI_PinballReactive OtherActor))
  (Default|PinballImpulseEvent _asbpi_pinball_reactive (* (Math|Vector|Normalize (- (Transformation|GetWorldLocation OtherComp) (Transformation|GetActorLocation))) (Variables|Default|GetBumpStrength)))
  (Development|PrintString "ygo;ihubhjku")
  (if (Utilities|DoesObjectImplementInterface _returnvalue "/Game/Assets/Blueprints/BPI_ScoreReciever.BPI_ScoreReciever_C")
    (Class|BPIScoreReciever|AddScore(Message) _returnvalue (Variables|Default|GetPointValue))))

(event EventTick
  (params (DeltaSeconds :type Float%20%28single-precision%29)))

(fn ConstructionScript)