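; Actor Blueprint for a left and right pair of flippers, apparently pinball-style, that swing on command.
; FlipL and FlipR play separate timelines that lerp each flipper's relative rotation toward opposite 90-degree targets, while UnflipL and UnflipR reverse them.
; BeginPlay takes the shared start rotation from the root component, sets both end rotations and raises timeline play rates for a fast snap.
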(event Custom|FlipL
  ;[0.15 0.15 0.15 0.5] Flips left flipper
  (bind _newtrack_0 (Timeline|Timeline_0 Play)
    (:Update
      (Transformation|SetRelativeRotation (Variables|Default|GetFlipper1) (Math|Rotator|Lerp(Rotator) (Variables|Default|GetStartRotation) (Variables|Default|GetEndRotationL) _newtrack_0) false false))))

(event Custom|FlipR
  ;[0.15 0.15 0.15 0.5] Flips right flipper
  (bind _newtrack_0 (Timeline|Timeline Play)
    (:Update
      (Transformation|SetRelativeRotation (Variables|Default|GetFlipper) (Math|Rotator|Lerp(Rotator) (Variables|Default|GetStartRotation) (Variables|Default|GetEndRotationR) _newtrack_0) false false))))

(event Custom|UnflipR
  ;[0.15 0.15 0.15 0.5] Flips right flipper
  (bind _newtrack_0 (Timeline|Timeline Reverse)
    (:Update
      (Transformation|SetRelativeRotation (Variables|Default|GetFlipper) (Math|Rotator|Lerp(Rotator) (Variables|Default|GetStartRotation) (Variables|Default|GetEndRotationR) _newtrack_0) false false))))

(event Custom|UnflipL
  ;[0.15 0.15 0.15 0.5] Flips left flipper
  (bind _newtrack_0 (Timeline|Timeline_0 Reverse)
    (:Update
      (Transformation|SetRelativeRotation (Variables|Default|GetFlipper1) (Math|Rotator|Lerp(Rotator) (Variables|Default|GetStartRotation) (Variables|Default|GetEndRotationL) _newtrack_0) false false))))

(event EventBeginPlay
  ;[0.15 0.15 0.15 0.5] Start and end rotation
  (Variables|Default|SetStartRotation (Variables|/Script/Engine.SceneComponent|GetRelativeRotation (Variables|Default|GetDefaultSceneRoot)))
  (Variables|Default|SetEndRotationR "0.000000,90.000000,0.000000")
  (Variables|Default|SetEndRotationL "0.000000,-90.000000,0.000000")
  ;[0.15 0.15 0.15 0.5] Speeds up flipping
  (Components|Timeline|SetPlayRate (Variables|Default|GetTimeline) 1e+01)
  (Components|Timeline|SetPlayRate (Variables|Default|GetTimeline_0) 1e+01))

(fn ConstructionScript)